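; Base weapon Blueprint with a hitscan Fire function, apparently an early debug implementation.
; Fire casts player character 0 to Ue4ASP_Character and runs a short Visibility line trace forward from its PlayerCamera, drawing persistent debug lines.
; A hit shows a placeholder on-screen message, while a play-sound call with no sound assigned runs at the hit location regardless of result.
; The event graph and construction script are empty.
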(fn `Fire`
  (bind _asue_4asp_character (cast `/Game/Blueprints/Ue4ASP_Character` (`GameplayStatics.GetPlayerCharacter` 0)))
  (bind _playercamera (`/Game/Blueprints/Ue4ASP_Character.PlayerCamera` _asue_4asp_character))
  (bind _returnvalue (`SceneComponent.K2_GetComponentLocation` _playercamera))
  (bind (_outhit _returnvalue_2) (`KismetSystemLibrary.LineTraceSingle` :`Start` _returnvalue :`End` (+ (* (`KismetMathLibrary.GetForwardVector` (`SceneComponent.K2_GetComponentRotation` _playercamera)) 1500.0) _returnvalue) :`TraceChannel` "TraceTypeQuery1" :`DrawDebugType` "Persistent"))
  (`KismetSystemLibrary.PrintString` "Hello" _returnvalue_2)
  (`GameplayStatics.PlaySoundAtLocation` null (`.Location` (`GameplayStatics.BreakHitResult` _outhit)) (struct) 1.0 1.0 0.0 null null null))

(fn `UserConstructionScript`)