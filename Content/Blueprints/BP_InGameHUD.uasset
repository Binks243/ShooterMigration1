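; BP_InGameHUD is an in-game HUD Blueprint that manages an item-overlap alert widget.
; On BeginPlay it creates WBP_ItemOverlappAlert for the first player controller, stores it, and adds it to the viewport hidden.
; AlertWidgetVisible and AlertWidgetHidden toggle that widget's visibility so other code can show or hide the alert.
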(event `self.ReceiveBeginPlay`
  (bind _returnvalue (`|CreateWidget` "/Game/Blueprints/WBP_ItemOverlappAlert.WBP_ItemOverlappAlert_C" (`GameplayStatics.GetPlayerController` 0)))
  (bind _output_get (set `self.ItemOverlapAlertWidget` _returnvalue))
  (`Widget.SetVisibility` _output_get "Hidden")
  (`UserWidget.AddToViewport` _returnvalue 0))

(fn `AlertWidgetHidden`
  (`Widget.SetVisibility` (`self.ItemOverlapAlertWidget`) "Hidden"))

(fn `AlertWidgetVisible`
  (`Widget.SetVisibility` (`self.ItemOverlapAlertWidget`) "Visible"))

(fn `UserConstructionScript`)